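; Laser component that fires a colored beam from the parent's Muzzle socket while ShouldTrace is set, bouncing it through the level.
; Each Tick, recursive LaserTraces notifies BPI_Laser actors or reflects off non-default physical surfaces, with SurfaceType2 prisms able to add a green branch.
; The resulting segments drive BP_NIagara beams and NS_Sparks impacts pooled at BeginPlay, hiding unused ones.
; Recursion has no depth limit; SpawnParticle functions appear unused.
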(event EventBeginPlay
  (bind _returnvalue (Game|SpawnActorfromClass "/Game/Lasery/LaserComponent/BP_NIagara.BP_NIagara_C" (Transformation|GetActorTransform (Components|GetOwner)) "Undefined" "MultiplyWithRoot" 0 "0.000000,0.000000,0.000000" 0))
  (Variables|Components|SetNS_LaserFromGun _returnvalue)
  (Transformation|AttachComponentToComponent _returnvalue self "None" "SnapToTarget" "SnapToTarget" "SnapToTarget" true)
  (bind _returnvalue_2 (Niagara|SpawnSystemAttached "/Game/Lasery/LaserComponent/VFX/NS_Sparks.NS_Sparks" self "None" "0, 0, 0" "0, 0, 0" "SnapToTarget" false))
  (Variables|Default|SetNS_ImpactFromGun _returnvalue_2)
  (for _index (range 1 (Variables|Default|GetMax_Niagara_Component_Count))
    (bind _returnvalue_3 (Game|SpawnActorfromClass "/Game/Lasery/LaserComponent/BP_NIagara.BP_NIagara_C" (Math|Transform|MakeTransform "0, 0, 0" "0, 0, 0" "1.000000,1.000000,1.000000") "Undefined" "MultiplyWithRoot" 0 "0.000000,0.000000,0.000000" 0))
    (Utilities|Array|Add (Variables|Components|GetNS_LaserActors) _returnvalue_3)
    (Rendering|SetActorHiddenInGame _returnvalue_3 true))
  (for _index_2 (range 1 (Variables|Default|GetMax_Niagara_Component_Count))
    (bind _returnvalue_4 (Niagara|SpawnSystematLocation "/Game/Lasery/LaserComponent/VFX/NS_Sparks.NS_Sparks" "0, 0, 0"))
    (Utilities|Array|Add (Variables|Components|GetNS_ImpactComps) _returnvalue_4)
    (Development|SetHiddeninGame _returnvalue_4 true false)))

(event EventTick
  (params (DeltaSeconds :type Float%20%28single-precision%29))
  (bind _ns_laseractors (Variables|Components|GetNS_LaserActors))
  (bind _ns_laserfromgun (Variables|Components|GetNS_LaserFromGun))
  (bind _ns_impactfromgun (Variables|Default|GetNS_ImpactFromGun))
  (bind _niagaracomponent (Variables|/Script/Niagara.NiagaraActor|GetNiagaraComponent _ns_laserfromgun))
  (Utilities|Array|Clear (Variables|Default|GetLineTraces))
  (Variables|Default|SetRecursive%20Iteration%20Count 0)
  (if (Variables|Public(Settedoutside)|GetShouldTrace)
    (bind (_outhit _returnvalue) (Collision|LineTraceByChannel (Transformation|GetSocketLocation (Transformation|GetAttachParent) "Muzzle") (+ (* (Math|Vector|GetForwardVector) (Variables|Default|GetLaserDistance)) (Transformation|GetActorLocation (Components|GetOwner))) "TraceTypeQuery3" false 0 "ForOneFrame" true "(R=1.000000,G=0.000000,B=0.000000,A=1.000000)" "(R=0.000000,G=1.000000,B=0.000000,A=1.000000)" 1.0))
    (Transformation|SetWorldLocation _ns_impactfromgun (.Location (Collision|BreakHitResult _outhit)) false false)
    (Development|SetHiddeninGame _ns_impactfromgun false false)
    (Rendering|SetActorHiddenInGame _ns_laserfromgun false)
    (Niagara|SetNiagaraVariable(Vector3) _niagaracomponent "LaserEnd" (select _returnvalue (.Location (Collision|BreakHitResult _outhit)) (.TraceEnd (Collision|BreakHitResult _outhit))))
    (Niagara|SetNiagaraVariable(LinearColor) _niagaracomponent "Color" (Variables|Public(Settedoutside)|GetLaserColor))
    (if _returnvalue
      (CallFunction|LaserTraces _outhit (Variables|Public(Settedoutside)|GetLaserColor))
      (for (_array_element _array_index) (Variables|Default|GetLineTraces)
        (bind _output (Utilities|ValidateGet (Variables|Components|GetNS_LaserActors) _array_index)
          (:Is%20Valid
            (Transformation|SetActorLocation _output (.LineStart (Utilities|Struct|BreakS_LineTrace _array_element)) false false)
            (Niagara|SetNiagaraVariable(Vector3) (Variables|/Script/Niagara.NiagaraActor|GetNiagaraComponent _output) "LaserEnd" (select (.DidItHit (Utilities|Struct|BreakS_LineTrace _array_element)) (.Location (Utilities|Struct|BreakS_LineTrace _array_element)) (.LineEnd (Utilities|Struct|BreakS_LineTrace _array_element))))
            (Niagara|SetNiagaraVariable(LinearColor) (Variables|/Script/Niagara.NiagaraActor|GetNiagaraComponent _output) "Color" (.LaserColor (Utilities|Struct|BreakS_LineTrace _array_element)))
            (Rendering|SetActorHiddenInGame _output false)
            (Utilities|IsValid (Utilities|Array|Get(acopy) (Variables|Components|GetNS_ImpactComps) _array_index)
              (:Is%20Valid
                (Transformation|SetWorldLocation (Utilities|Array|Get(acopy) (Variables|Components|GetNS_ImpactComps) _array_index) (.Location (Utilities|Struct|BreakS_LineTrace _array_element)) false false)
                (Development|SetHiddeninGame (Utilities|Array|Get(acopy) (Variables|Components|GetNS_ImpactComps) _array_index) false false)
                (Niagara|SetNiagaraVariable(LinearColor) (Utilities|Array|Get(acopy) (Variables|Components|GetNS_ImpactComps) _array_index) "Color" (.LaserColor (Utilities|Struct|BreakS_LineTrace _array_element))))))
          (:Is%20Not%20Valid
            (Development|PrintString "Niagara Actor NOTTTT VALID"))))
      (for _index (range (Utilities|Array|Length (Variables|Default|GetLineTraces)) (- (Utilities|Array|Length _ns_laseractors) 1))
        (bind _output_2 (Utilities|ValidateGet _ns_laseractors _index)
          (:Is%20Valid
            (Rendering|SetActorHiddenInGame _output_2 true)
            (Utilities|IsValid (Utilities|Array|Get(acopy) (Variables|Components|GetNS_ImpactComps) _index)
              (:Is%20Valid
                (Development|SetHiddeninGame (Utilities|Array|Get(acopy) (Variables|Components|GetNS_ImpactComps) _index) true false))))))
      (else
        (for _array_element_2 (Variables|Components|GetNS_LaserActors)
          (Rendering|SetActorHiddenInGame _array_element_2 true)
          (for _array_element_3 (Variables|Components|GetNS_ImpactComps)
            (Development|SetHiddeninGame _array_element_3 true false)))))
    (else
      (Development|SetHiddeninGame (Variables|Default|GetNS_ImpactFromGun) true true)
      (Rendering|SetActorHiddenInGame (Variables|Components|GetNS_LaserFromGun) true)
      (for _array_element_4 (Variables|Components|GetNS_LaserActors)
        (Rendering|SetActorHiddenInGame _array_element_4 true)
        (for _array_element_5 (Variables|Components|GetNS_ImpactComps)
          (Development|SetHiddeninGame _array_element_5 true false))))))

(fn LaserTraces
  (params (Hit :type Hit%20Result%20Structure%20%28by%20ref%29) (LaserColor :type Linear%20Color%20Structure :default "(R=0.596078,G=0.019608,B=0.000000,A=1.000000)"))
  (bind (_bblockinghit _binitialoverlap _time _distance _location _impactpoint _normal _impactnormal _physmat _hitactor _hitcomponent _hitbonename _bonename _hititem _elementindex _faceindex _tracestart _traceend) (Collision|BreakHitResult Hit))
  (bind _returnvalue (Utilities|IsValid _physmat))
  (bind _returnvalue_2 (- _traceend _tracestart))
  (bind _surfacetype (Variables|/Script/PhysicsCore.PhysicalMaterial|GetSurfaceType _physmat))
  (bind _returnvalue_3 (select _returnvalue _surfacetype "SurfaceType_Default"))
  (LocalVariables|SetLineColor LaserColor)
  (LocalVariables|SetPreviousHit Hit)
  (if (Utilities|DoesObjectImplementInterface _hitactor "/Game/Lasery/LaserComponent/BPI_Laser.BPI_Laser_C")
    (Class|BPILaser|OnLaserHit(Message) _hitactor (LocalVariables|GetLineColor))
    (elif (Utilities|Enum|NotEqual(Enum) _returnvalue_3 "SurfaceType_Default")
      (bind (_outhit _returnvalue_4) (Collision|LineTraceByChannel _location (+ _location (- _returnvalue_2 (* (* (Math|Vector|DotProduct _returnvalue_2 _normal) 2.0) _normal))) "TraceTypeQuery3" false (Utilities|Array|MakeArray _hitactor) "ForOneFrame" true "(R=0.000000,G=0.346492,B=1.000000,A=1.000000)" "(R=1.000000,G=0.000000,B=0.630471,A=1.000000)" 1.0))
      (LocalVariables|SetLineTrace (Utilities|Struct|MakeS_LineTrace (.TraceStart (Collision|BreakHitResult _outhit)) (.TraceEnd (Collision|BreakHitResult _outhit)) (.Location (Collision|BreakHitResult _outhit)) _returnvalue_4 (LocalVariables|GetLineColor)))
      (Utilities|Array|Add (Variables|Default|GetLineTraces) (LocalVariables|GetLineTrace))
      (if (.didithit (LocalVariables|GetLineTrace))
        (Math|Integer|IncrementInt (Variables|Default|GetRecursive%20Iteration%20Count)
          (:%20%20
            (CallFunction|LaserTraces _outhit (.lasercolor (LocalVariables|GetLineTrace)))
            ;[0.2645 1 0.3567] Prism
            (if (Utilities|Enum|Equal(Enum) _returnvalue_3 "SurfaceType2")
              (bind (_outhit_2 _returnvalue_5) (Collision|LineTraceByChannel (.TraceStart (Collision|BreakHitResult _outhit)) (Math|Vector|MakeVector (* (.x (.TraceEnd (Collision|BreakHitResult _outhit))) -1.0) (* (.y (.TraceEnd (Collision|BreakHitResult _outhit))) -1.0) (.z (.TraceEnd (Collision|BreakHitResult _outhit)))) "TraceTypeQuery3" false (Utilities|Array|MakeArray (.HitActor (Collision|BreakHitResult _outhit)) (.HitActor (Collision|BreakHitResult (LocalVariables|GetPreviousHit)))) "ForOneFrame" true "(R=1.000000,G=0.669267,B=0.000000,A=1.000000)" "(R=1.000000,G=0.000000,B=0.630471,A=1.000000)" 1.0))
              (Utilities|Array|Add (Variables|Default|GetLineTraces) (Utilities|Struct|MakeS_LineTrace (.TraceStart (Collision|BreakHitResult _outhit_2)) (.TraceEnd (Collision|BreakHitResult _outhit_2)) (.Location (Collision|BreakHitResult _outhit_2)) _returnvalue_5 (.green (Variables|Default|GetColors))))
              (if _returnvalue_5
                (Math|Integer|IncrementInt (Variables|Default|GetRecursive%20Iteration%20Count)
                  (:%20%20
                    (CallFunction|LaserTraces _outhit_2 (.green (Variables|Default|GetColors)))))))))))))

(fn SpawnParticle
  (params (LineTrace :type S%20Line%20Trace%20Structure))
  (bind (_linestart _lineend _location _didithit) (Utilities|Struct|BreakS_LineTrace LineTrace))
  (bind _returnvalue (Game|SpawnActorfromClass "/Game/Lasery/LaserComponent/BP_NIagara.BP_NIagara_C" (Math|Transform|MakeTransform _linestart "0, 0, 0" "1.000000,1.000000,1.000000") "Undefined" "MultiplyWithRoot" 0 (select _didithit _location _lineend) 0))
  (return _returnvalue))

(fn SpawnParticleOld
  (params (Hit :type Hit%20Result%20Structure%20%28by%20ref%29) (Index :type Boolean) (LineTrace :type S%20Line%20Trace%20Structure))
  (bind (_bblockinghit _binitialoverlap _time _distance _location _impactpoint _normal _impactnormal _physmat _hitactor _hitcomponent _hitbonename _bonename _hititem _elementindex _faceindex _tracestart _traceend) (Collision|BreakHitResult Hit))
  (bind _ns_laseractors (Variables|Components|GetNS_LaserActors))
  (bind _recursive_iteration_count (Variables|Default|GetRecursive%20Iteration%20Count))
  (bind _output (Utilities|Array|Get(acopy) _ns_laseractors _recursive_iteration_count))
  (bind _returnvalue (Game|SpawnActorfromClass "/Game/Lasery/LaserComponent/BP_NIagara.BP_NIagara_C" (Math|Transform|MakeTransform _tracestart "0, 0, 0" "1.000000,1.000000,1.000000") "Undefined" "MultiplyWithRoot" 0 (select Index "0, 0, 0" _traceend) 0))
  (Utilities|IsValid _output
    (:Is%20Valid
      (Actor|DestroyActor _output))
    (:Is%20Not%20Valid
      _))
  (Utilities|Array|Insert (Variables|Components|GetNS_LaserActors) _returnvalue (Variables|Default|GetRecursive%20Iteration%20Count)))