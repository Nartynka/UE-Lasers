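; BP_Target is a laser target that is hit successfully only by a laser of its assigned color.
; The construction script applies the material from its Color object to the cylinder mesh when that reference is valid.
; OnLaserHit compares the incoming color to the assigned one; a match calls OnTargetHit, prints a win message and destroys the actor, while a mismatch only prints a warning.
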(event EventOnLaserHit
  (params (LaserColor :type Linear%20Color%20Structure))
  (if (== LaserColor (Variables|/Game/Lasery/PDA_Colors.PDA_Colors_C|GetColor (Variables|Default|GetColor)))
    (Default|CallOnTargetHit)
    (Development|PrintString "WINNNNNN!!" true true "(R=0.047914,G=1.000000,B=0.158916,A=1.000000)" 2.0 "")
    (Actor|DestroyActor)
    (else
      (Development|PrintString "Wrong Laser Color!" true true "(R=0.043423,G=0.176825,B=1.000000,A=1.000000)"))))

(fn ConstructionScript
  (bind _color (Variables|Default|GetColor)
    (:then
      (Rendering|Material|SetMaterial (Variables|Default|GetCylinder) 0 (Variables|/Game/Lasery/PDA_Colors.PDA_Colors_C|GetMaterial _color)))
    (:else)))