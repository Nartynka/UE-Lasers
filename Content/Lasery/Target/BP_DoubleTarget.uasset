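; BP_DoubleTarget is a laser target that reports to a Parent object when hit by a laser of its own color.
; OnLaserHit compares the laser color to the target's Color and passes itself to Parent.TargetHit, or prints a wrong-color message.
; Activation is a separate event that fires the OnTargetHit dispatcher, prints the color name and destroys the actor.
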(event Custom|Activate
  (Default|CallOnTargetHit)
  (Development|PrintString (Utilities|String|ToString(Name) (Variables|/Game/Lasery/PDA_Colors.PDA_Colors_C|GetName (Variables|Default|GetColor))) true true "(R=0.047914,G=1.000000,B=0.158916,A=1.000000)" 2.0 "")
  (Actor|DestroyActor))

(event EventBeginPlay)

(event Collision|EventActorBeginOverlap
  (params (OtherActor :type Actor%20Object%20Reference)))

(event EventTick
  (params (DeltaSeconds :type Float%20%28single-precision%29)))

(event EventOnLaserHit
  (params (LaserColor :type Linear%20Color%20Structure))
  (if (== LaserColor (Variables|/Game/Lasery/PDA_Colors.PDA_Colors_C|GetColor (Variables|Default|GetColor)))
    (Default|TargetHit (Variables|Default|GetParent) self)
    (else
      (Development|PrintString "Wrong Laser Color!" true true "(R=0.043423,G=0.176825,B=1.000000,A=1.000000)"))))

(fn ConstructionScript
  (|CallParentFunction))