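; BP_Emitter is a laser emitter actor that passes its ShouldEmitLaser flag to BPLaserComponent on BeginPlay to control tracing.
; Its LaserTrace function, not called here, recursively line-traces reflections off hit normals, draws debug beams and sends OnLaserHitMessage to hit actors.
; The recursion limit logic is disconnected, so bounces end only when a trace misses.
; A stray NewFunction computes a forward segment from a hit actor.
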(event EventBeginPlay
  (Variables|/Game/Lasery/LaserComponent/BP_Laser_Component.BP_Laser_Component_C|SetShouldTrace (Variables|Default|GetBP_Laser_Component) (Variables|Default|GetShouldEmitLaser)))

(fn ConstructionScript)

(fn NewFunction
  (params (Hit :type Hit%20Result%20Structure%20%28by%20ref%29))
  (bind _hitactor (Collision|BreakHitResult Hit))
  (bind _returnvalue (Transformation|GetActorLocation _hitactor))
  (return _returnvalue (+ _returnvalue (* 1e+03 (Transformation|GetActorForwardVector _hitactor)))))

(fn LaserTrace
  (params (Hit :type Hit%20Result%20Structure%20%28by%20ref%29))
  (bind (_bblockinghit _binitialoverlap _time _distance _location _impactpoint _normal _impactnormal _physmat _hitactor _hitcomponent _hitbonename _bonename _hititem _elementindex _faceindex _tracestart _traceend) (Collision|BreakHitResult Hit))
  (bind _returnvalue (- _traceend _tracestart))
  (bind (_outhit _returnvalue_2) (Collision|LineTraceByChannel _location (+ _location (- _returnvalue (* (* (Math|Vector|DotProduct _returnvalue _normal) 2.0) _normal))) "TraceTypeQuery3" false (Utilities|Array|MakeArray _hitactor) "ForOneFrame" true "(R=0.000000,G=0.346492,B=1.000000,A=1.000000)" "(R=1.000000,G=0.000000,B=0.630471,A=1.000000)"))
  (Class|BPILaser|OnLaserHit(Message) (.HitActor (Collision|BreakHitResult _outhit)))
  (if _returnvalue_2
    (CallFunction|LaserTrace _outhit)))