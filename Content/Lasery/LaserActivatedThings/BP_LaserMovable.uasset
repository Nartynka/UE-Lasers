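; BP_LaserMovable is a laser puzzle object that slides its cube to MoveToLocation once its linked targets report hits.
; On BeginPlay it binds to up to three targets' OnTargetHit events, pre-setting a flag for each missing optional target.
; Each hit sets the next unset flag, regardless of which target fired; once both are set, a hit plays a Timeline lerping the cube's relative location from zero.
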(event Custom|ChangeShouldActivate
  (if (Variables|Default|GetShouldActivate)
    (if (Variables|Default|GetShouldActivate_2)
      (CallFunction|Move)
      (else
        (Variables|Default|SetShouldActivate_2 true)))
    (else
      (Variables|Default|SetShouldActivate true))))

(event Custom|Move
  (Utilities|FlowControl|Sequence
    (:then_0
      (bind _alpha (Timeline|Timeline Play)
        (:Update
          (Transformation|SetRelativeLocation (Variables|Default|GetCube) (Math|Vector|Lerp(Vector) "0, 0, 0" (Variables|Default|GetMoveToLocation) _alpha) false false))))))

(event EventBeginPlay
  (bind _target (Variables|Default|GetTarget)
    (:then
      (EventDispatchers|BindEventtoOnTargetHit _target (delegate Custom|ChangeShouldActivate))
      (bind _target_2 (Variables|Default|GetTarget_2)
        (:then
          (EventDispatchers|BindEventtoOnTargetHit _target_2 (delegate Custom|ChangeShouldActivate)))
        (:else
          (Variables|Default|SetShouldActivate true)))
      (bind _target_3 (Variables|Default|GetTarget_3)
        (:then
          (EventDispatchers|BindEventtoOnTargetHit _target_3 (delegate Custom|ChangeShouldActivate)))
        (:else
          (Variables|Default|SetShouldActivate_2 true))))
    (:else
      (Development|PrintString "Target is not Valid!!!" true true "(R=1.000000,G=0.046926,B=0.000000,A=1.000000)"))))

(fn ConstructionScript)